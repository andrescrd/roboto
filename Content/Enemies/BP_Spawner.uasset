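; BP_Spawner continually spawns randomized BP_Shape actors within a spawn area and clears those reaching a destroy area.
; Tick drives a DoOnce gate that resets after a SpawnerTime delay, spacing out spawns.
; Each shape gets a random position, per-axis scale and mesh, plus a random dynamic material instance with a random EnemyColor.
; DestroyArea overlaps trigger the destroy event on any BP_Shape.
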(event `self.ReceiveTick`
  (params (DeltaSeconds :type "Float (single-precision)"))
  (bind _returnvalue (`KismetMathLibrary.RandomFloatInRange` 1.0 2.5))
  (bind (_origin _boxextent) (`KismetSystemLibrary.GetComponentBounds` (`self.SpawnArea`)))
  (`/Engine/EditorBlueprintResources/StandardMacros.DoOnce` false :!label _label
    (:`Completed`
      (`|ExecutionSequence`
        (:`then_0`
          ;[1 0.8987 0.3411] Spanw shape with random rotation in random place of spawn area
          (bind _returnvalue_2 (`|SpawnActorFromClass` "/Game/Enemies/BP_Shape.BP_Shape_C" (`KismetMathLibrary.MakeTransform` (`KismetMathLibrary.RandomPointInBoundingBox` _origin _boxextent) (struct) (`KismetMathLibrary.MakeVector` _returnvalue _returnvalue _returnvalue)) "Undefined" "OverrideRootScale" null null))
          (bind _staticmesh (`/Game/Enemies/BP_Shape.StaticMesh` _returnvalue_2))
          ;[0.1602 1 0.3842] Set random mesh to shape
          (`StaticMeshComponent.SetStaticMesh` _staticmesh (select `int` (`KismetMathLibrary.RandomIntegerInRange` 0 3) :`0` "/Game/Enemies/Meshes/Shape_Torus.Shape_Torus" :`1` "/Game/Enemies/Meshes/SM_SpikeEnemy.SM_SpikeEnemy" :`2` "/Game/Enemies/Meshes/SM_StarEnemy.SM_StarEnemy" :`3` "/Game/Enemies/Meshes/SM_StarEnemyChild.SM_StarEnemyChild" :!type "StaticMesh Object Reference"))
          ;[0.2168 0.8192 1] Set random material to shape
          (bind _returnvalue_3 (`PrimitiveComponent.CreateDynamicMaterialInstance` _staticmesh 0 (select `int` (`KismetMathLibrary.RandomIntegerInRange` 0 3) :`0` "/Game/Enemies/Materials/MI_RedEnemy_Pulse.MI_RedEnemy_Pulse" :`1` "/Game/Enemies/Materials/MI_WireframeMaster_NoPulse.MI_WireframeMaster_NoPulse" :`2` "/Game/Enemies/Materials/MI_RedEnemy_WF.MI_RedEnemy_WF" :`3` "/Game/Enemies/Materials/M_MasterEnemy.M_MasterEnemy" :!type "MaterialInterface Object Reference") "None"))
          ;[1 0.1521 0.2319] Set random color to shape
          (`MaterialInstanceDynamic.SetVectorParameterValue` _returnvalue_3 "EnemyColor" (`KismetMathLibrary.MakeColor` (`KismetMathLibrary.RandomFloat`) (`KismetMathLibrary.RandomFloat`) (`KismetMathLibrary.RandomFloat`))))
        (:`then_1`
          (`KismetSystemLibrary.Delay` (`self.SpawnerTime`))
          (goto _label :!via `Reset`))))))

(event `self.DestroyArea.OnComponentBeginOverlap`
  (params (OverlappedComponent :type "PrimitiveComponent Object Reference") (OtherActor :type "Actor Object Reference") (OtherComp :type "PrimitiveComponent Object Reference") (OtherBodyIndex :type Integer) (bFromSweep :type Boolean) (SweepResult :type "HitResult Structure (by ref)"))
  ;[0.0582 0.05294 1] Destroy Shapes taht touch te destroy area
  (bind _asbp_shape (cast `/Game/Enemies/BP_Shape` OtherActor))
  (`/Game/Enemies/BP_Shape.EventDestroy` _asbp_shape))

(fn `UserConstructionScript`)
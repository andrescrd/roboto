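; BP_Roboto_Blue is an enemy robot that spins its base and shoots at a given actor with hitscan fire.
; Tick rotates Base by a fixed step every frame, independent of delta time.
; EventShoot plays an explosion emitter at ProjectileSpawner, then runs a debug-drawn Visibility trace from the actor's location to the target.
; Fixed damage applies only when the trace hits that target first, so obstacles block shots.
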(event `self.ReceiveTick`
  (params (DeltaSeconds :type "Float (single-precision)"))
  (`SceneComponent.K2_AddRelativeRotation` (`self.Base`) (struct :`Yaw` 45.0) false false))

(event `EventShoot`
  (params (EnemyToShoot :type "Actor Object Reference"))
  ;[1 0.2384 0.2783] Shoot to any actor
  (`self.EventPlayShootFx`)
  (bind (_outhit _returnvalue) (`KismetSystemLibrary.LineTraceSingle` :`Start` (`self.K2_GetActorLocation`) :`End` (`self.K2_GetActorLocation` EnemyToShoot) :`TraceChannel` "TraceTypeQuery1" :`DrawDebugType` "ForDuration"))
  (if _returnvalue
    (bind (_bblockinghit _binitialoverlap _time _distance _location _impactpoint _normal _impactnormal _physmat _hitactor) (`GameplayStatics.BreakHitResult` _outhit))
    (if (== _hitactor EnemyToShoot)
      (`GameplayStatics.ApplyDamage` _hitactor 20.0))))

(event `EventPlayShootFx`
  (bind _projectilespawner (`self.ProjectileSpawner`))
  ;[0.6531 1 0.2066] Play Effect when shoot
  (`GameplayStatics.SpawnEmitterAtLocation` "/Game/MobileStarterContent/Particles/P_Explosion.P_Explosion" (`SceneComponent.K2_GetComponentLocation` _projectilespawner) (`SceneComponent.K2_GetComponentRotation` _projectilespawner)))

(fn `UserConstructionScript`)
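; BP_MovableBox is a movable prop whose Disc component can slide toward an EndPoint component and spin, each behavior toggled by a flag.
; The construction script stores Disc's world location as the start point.
; Tick lerps Disc to EndPoint using the MovementTime timeline's value, though nothing here plays that timeline.
; Tick also adds SpeedRotation as local yaw each frame, without delta-time scaling.
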(event Custom|EventRotation
  ;[1 0.224 0.224] Setup Rotation
  (if (Variables|Default|GetEnableRotator)
    (Transformation|AddLocalRotation (Variables|Components|GetDisc) (Math|Rotator|MakeRotator 0.0 0.0 (Variables|Default|GetSpeedRotation)) false false)))

(event Custom|EventMovement
  ;[0.6663 1 0.6413] Setup Movement
  (if (Variables|Default|GetAutoStart)
    (Transformation|SetWorldLocation (Variables|Components|GetDisc) (Math|Vector|Lerp(Vector) (.location (Variables|Default|GetStartPoint)) (Transformation|GetWorldLocation (Variables|Default|GetEndPoint)) (stale _time)) false false)))

(event EventTick
  (params (DeltaSeconds :type Float%20%28single-precision%29))
  (CallFunction|EventMovement)
  (CallFunction|EventRotation))

(fn ConstructionScript
  (Variables|Default|SetStartPoint (Math|Conversions|ToTransform(Vector) (Transformation|GetWorldLocation (Variables|Components|GetDisc)))))
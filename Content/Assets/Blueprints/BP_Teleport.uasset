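; Teleport actor that, when flagged as the end teleport, loads a named level once the player has collected enough items.
; On BeginPlay, the end teleport calls Activate without reset on both aura components, although the author's note describes deactivation.
; Trigger box overlap checks BP_Player's item counter against the required count, then opens the level or prints a hint to get more items.
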(event `self.ReceiveBeginPlay`
  ;[1 0.6079 0.7189] If end teleport particles are deactivate
  (if (`self.IsEndTeleport`)
    (`ActorComponent.Activate` (`self.Aura`) false)
    (`ActorComponent.Activate` (`self.Aura2`) false)))

(event `self.TriggerBox.OnComponentBeginOverlap`
  (params (OverlappedComponent :type "PrimitiveComponent Object Reference") (OtherActor :type "Actor Object Reference") (OtherComp :type "PrimitiveComponent Object Reference") (OtherBodyIndex :type Integer) (bFromSweep :type Boolean) (SweepResult :type "HitResult Structure (by ref)"))
  ;[0.1667 1 1] Overlap when player enter to telleport
  (if (`self.IsEndTeleport`)
    (bind _asbp_player (cast `/Game/PlayerBP/Blueprints/BP_Player` OtherActor))
    (if (>= (`/Game/PlayerBP/Blueprints/BP_Player.ItemCounter` _asbp_player) (`self.ItemsForOpenTeleport`))
      (`GameplayStatics.OpenLevel` (`self.LevelName`))
      (else
        (`KismetSystemLibrary.PrintString` "Try to get more items")))))

(fn `UserConstructionScript`)
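; BP_Shape is a falling enemy shape that can spin and explode.
; Tick moves it down the world Z axis at FallSpeed, scaled by delta time, with sweep enabled.
; When RandomRotation is set, BeginPlay gives its RotatingMovement component a random rotation rate without roll.
; EventDestroy spawns the P_Explosion emitter at its location, then destroys the actor; nothing in this graph calls it.
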(event `self.ReceiveTick`
  (params (DeltaSeconds :type "Float (single-precision)"))
  ;[1 0.166 0.2959] Setup Fall Speed
  (`self.K2_AddActorWorldOffset` (`KismetMathLibrary.MakeVector` 0.0 0.0 (* (* DeltaSeconds (`self.FallSpeed`)) -1.0)) true))

(event `self.ReceiveBeginPlay`
  ;[0.3228 0.31 1] Setup Random Rotation
  (if (`self.RandomRotation`)
    (set `RotatingMovementComponent.RotationRate` (`KismetMathLibrary.RandomRotator` false) (`self.RotatingMovement`))))

(event `EventDestroy`
  ;[1 0.6804 0.202] Destroy Actor
  (`GameplayStatics.SpawnEmitterAtLocation` "/Game/MobileStarterContent/Particles/P_Explosion.P_Explosion" (`self.K2_GetActorLocation`))
  (`self.K2_DestroyActor`))

(fn `UserConstructionScript`)
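; BP_Spawner repeatedly spawns randomized BP_Shape enemies inside its SpawnArea bounds and clears them when they reach its DestroyArea.
; Tick drives a DoOnce gate that resets after a SpawnerTime delay, acting as a repeating spawn timer.
; Each shape gets a random location, per-axis scale, mesh and material, with a dynamic material instance randomizing EnemyColor.
; Shapes overlapping DestroyArea receive their EventDestroy call.
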(event `self.ReceiveTick`
  (params (DeltaSeconds :type "Float (single-precision)"))
  (bind _returnvalue (`KismetMathLibrary.RandomFloatInRange` 1.0 2.5))
  (bind (_origin _boxextent) (`KismetSystemLibrary.GetComponentBounds` (`self.SpawnArea`)))
  (`/Engine/EditorBlueprintResources/StandardMacros.DoOnce` false :!label _label
    (:`Completed`
      (`|ExecutionSequence`
        (:`then_0`
          (bind _returnvalue_2 (`|SpawnActorFromClass` "/Game/Enemy/BP_Shape.BP_Shape_C" (`KismetMathLibrary.MakeTransform` (`KismetMathLibrary.RandomPointInBoundingBox` _origin _boxextent) (struct) (`KismetMathLibrary.MakeVector` _returnvalue _returnvalue _returnvalue)) "Undefined" "OverrideRootScale" null null))
          (bind _staticmesh (`/Game/Enemy/BP_Shape.StaticMesh` _returnvalue_2))
          (`StaticMeshComponent.SetStaticMesh` _staticmesh (select `int` (`KismetMathLibrary.RandomIntegerInRange` 0 3) :`0` "/Game/Enemy/Meshes/Shape_Torus.Shape_Torus" :`1` "/Game/Enemy/Meshes/SM_SpikeEnemy.SM_SpikeEnemy" :`2` "/Game/Enemy/Meshes/SM_StarEnemy.SM_StarEnemy" :`3` "/Game/Enemy/Meshes/SM_StarEnemyChild.SM_StarEnemyChild" :!type "StaticMesh Object Reference"))
          (bind _returnvalue_3 (`PrimitiveComponent.CreateDynamicMaterialInstance` _staticmesh 0 (select `int` (`KismetMathLibrary.RandomIntegerInRange` 0 3) :`0` "/Game/Enemy/Materials/MI_RedEnemy_Pulse.MI_RedEnemy_Pulse" :`1` "/Game/Enemy/Materials/MI_WireframeMaster_NoPulse.MI_WireframeMaster_NoPulse" :`2` "/Game/Enemy/Materials/MI_RedEnemy_WF.MI_RedEnemy_WF" :`3` "/Game/Enemy/Materials/M_MasterEnemy.M_MasterEnemy" :!type "MaterialInterface Object Reference") "None"))
          (`MaterialInstanceDynamic.SetVectorParameterValue` _returnvalue_3 "EnemyColor" (`KismetMathLibrary.MakeColor` (`KismetMathLibrary.RandomFloat`) (`KismetMathLibrary.RandomFloat`) (`KismetMathLibrary.RandomFloat`))))
        (:`then_1`
          (`KismetSystemLibrary.Delay` (`self.SpawnerTime`))
          (goto _label :!via `Reset`))))))

(event `self.DestroyArea.OnComponentBeginOverlap`
  (params (OverlappedComponent :type "PrimitiveComponent Object Reference") (OtherActor :type "Actor Object Reference") (OtherComp :type "PrimitiveComponent Object Reference") (OtherBodyIndex :type Integer) (bFromSweep :type Boolean) (SweepResult :type "HitResult Structure (by ref)"))
  (bind _asbp_shape (cast `/Game/Enemy/BP_Shape` OtherActor))
  (`/Game/Enemy/BP_Shape.EventDestroy` _asbp_shape))

(fn `UserConstructionScript`)
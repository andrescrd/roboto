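; MyGameMode is a game mode that pulls the player camera boom to a new distance when triggered by BP_ChangeDirection actors.
; On BeginPlay it caches the BP_Player and its starting arm length, then binds its MoveCamera event to every BP_ChangeDirection in the level.
; MoveCamera plays a timeline that lerps the spring arm length from the starting distance to a fixed target.
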(event `self.ReceiveBeginPlay`
  ;[0.08493 0.6527 1] Get player reference
  (set `self.PlayerReference` (cast `/Game/PlayerBP/Blueprints/BP_Player` (`GameplayStatics.GetPlayerCharacter` 0) :!pure true))
  ;[0.04575 0.1431 1] Get start camera distance
  (set `self.InitialCameraDistance` (`SpringArmComponent.TargetArmLength` (`/Game/PlayerBP/Blueprints/BP_Player.CameraBoom` (`self.PlayerReference`))))
  (bind _outactors (`GameplayStatics.GetAllActorsOfClass` "/Game/Triggers/BP_ChangeDirection.BP_ChangeDirection_C"))
  (for _array_element _outactors
    (add `/Game/Triggers/BP_ChangeDirection.MoveCamera` _array_element (delegate `MoveCamera`))))

(event `MoveCamera`
  (bind (_direction _movement) (`Timeline|Timeline_0`)
    (:`Update`
      (set `SpringArmComponent.TargetArmLength` (`KismetMathLibrary.Lerp` (`self.InitialCameraDistance`) 800.0 _movement) (`/Game/PlayerBP/Blueprints/BP_Player.CameraBoom` (`self.PlayerReference`))))))

(fn `UserConstructionScript`)